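; Target dummy actor that shows where it takes point damage and how much, as a debugging aid.
; On point damage it stores the hit location and amount, then draws a short-lived debug sphere and damage number there.
; It then calls a custom event that repeats the same drawing from the stored values, only on the Remote branch of an authority switch.
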(event `self.ReceivePointDamage`
  (params (Damage :type "Float (single-precision)") (DamageType :type "DamageType Object Reference") (HitLocation :type "Vector Structure") (HitNormal :type "Vector Structure") (HitComponent :type "PrimitiveComponent Object Reference") (BoneName :type Name) (ShotFromDirection :type "Vector Structure") (InstigatedBy :type "Controller Object Reference") (DamageCauser :type "Actor Object Reference") (HitInfo :type "HitResult Structure (by ref)"))
  (set `self.Hit Location` HitLocation)
  (set `self.DamageMade` Damage)
  (`KismetSystemLibrary.DrawDebugSphere` (`self.Hit Location`) 3.0 12 (struct :`R` 0.062801 :`B` 1.0 :`A` 1.0) 1.0 2.0)
  (`KismetSystemLibrary.DrawDebugString` (`self.Hit Location`) (`KismetStringLibrary.Conv_DoubleToString` (`self.DamageMade`)) null (struct :`R` 1.0 :`G` 1.0 :`B` 1.0 :`A` 1.0) 1.0)
  (`self.EventReplicateDebugThings`))

(event `EventReplicateDebugThings`
  (bind _hit_location (`self.Hit Location`))
  (`/Engine/EditorBlueprintResources/ActorMacros.Switch Has Authority`
    (:`Remote`
      (`KismetSystemLibrary.DrawDebugSphere` _hit_location 3.0 12 (struct :`R` 0.062801 :`B` 1.0 :`A` 1.0) 1.0 2.0)
      (`KismetSystemLibrary.DrawDebugString` _hit_location (`KismetStringLibrary.Conv_DoubleToString` (`self.DamageMade`)) null (struct :`R` 1.0 :`G` 1.0 :`B` 1.0 :`A` 1.0) 1.0))))

(fn `UserConstructionScript`)