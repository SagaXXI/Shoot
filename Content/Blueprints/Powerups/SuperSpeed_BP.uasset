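; SuperSpeed powerup that temporarily doubles the walk speed of the player who activates it.
; OnActivated stores that player and multiplies the MaxWalkSpeed on their CharacterMovementComponent by two.
; OnExpired halves the current value if the stored player is still valid, rather than restoring a saved speed, then calls the parent's OnExpired.
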(event `self.OnActivated`
  (params (ActivatedForPlayer :type "Actor Object Reference"))
  (bind _returnvalue (`self.GetComponentByClass` ActivatedForPlayer "/Script/Engine.CharacterMovementComponent"))
  (set `self.ActivatePowerupTo` ActivatedForPlayer)
  (set `CharacterMovementComponent.MaxWalkSpeed` (* (`CharacterMovementComponent.MaxWalkSpeed` _returnvalue) 2.0) _returnvalue))

(event `self.OnExpired`
  (bind _activatepowerupto (`self.ActivatePowerupTo`))
  (bind _returnvalue (`self.GetComponentByClass` _activatepowerupto "/Script/Engine.CharacterMovementComponent"))
  (`/Engine/EditorBlueprintResources/StandardMacros.IsValid` _activatepowerupto
    (:`Is Valid`
      (set `CharacterMovementComponent.MaxWalkSpeed` (/ (`CharacterMovementComponent.MaxWalkSpeed` _returnvalue) 2.0) _returnvalue))
    (:`Is Not Valid`
      _))
  (`parent.OnExpired`))

(fn `UserConstructionScript`)