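; Powerup Blueprint that gives the activating player effectively infinite ammo while it is active.
; On activation it stores the player, casts it to SCharacter and sets the current weapon's loaded ammo to a very large number.
; On expiry it sets the then-current weapon's loaded ammo to a fixed normal amount, not the earlier count, then calls the parent's expiry logic.
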(event `self.OnActivated`
  (params (ActivatedForPlayer :type "Actor Object Reference"))
  (set `self.ActivateToPlayer` ActivatedForPlayer)
  (bind _asscharacter (cast `SCharacter` ActivatedForPlayer))
  (`Weapon.SetLoadedAmmo` (`SCharacter.CurrentWeapon` _asscharacter) 10000))

(event `self.OnExpired`
  (bind _asscharacter (cast `SCharacter` (`self.ActivateToPlayer`)))
  (`Weapon.SetLoadedAmmo` (`SCharacter.CurrentWeapon` _asscharacter) 30)
  (`parent.OnExpired`))

(fn `UserConstructionScript`
  (`parent.UserConstructionScript`))